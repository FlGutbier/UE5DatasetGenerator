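; BP_Config is a startup configuration actor that seeds a dataset run and launches its first level.
; On BeginPlay it sets console variables for local fog start distance, frame rate cap and texture streaming pool.
; It copies its level, actor, fog, material, camera position and light color settings into Dataset_GameInstance, so they persist across level loads.
; It then resets the index to zero and opens the first level in the list.
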(event `self.ReceiveBeginPlay`
  (`KismetSystemLibrary.ExecuteConsoleCommand` "r.LocalFogVolume.GlobalStartDistance 0" null)
  (`KismetSystemLibrary.ExecuteConsoleCommand` "t.MaxFps 240" null)
  (`KismetSystemLibrary.ExecuteConsoleCommand` "r.streaming.poolsize 10000" null)
  (bind _asdataset_game_instance (cast `/DatasetRendererBachelorThesis/Dataset_GameInstance` (`GameplayStatics.GetGameInstance`)))
  (bind _output_get (set `/DatasetRendererBachelorThesis/Dataset_GameInstance.Levels` (`self.Levels`) _asdataset_game_instance))
  (set `/DatasetRendererBachelorThesis/Dataset_GameInstance.ActorClass` (`self.Actors`) _asdataset_game_instance)
  (set `/DatasetRendererBachelorThesis/Dataset_GameInstance.AddFog` (`self.EnableFog`) _asdataset_game_instance)
  (set `/DatasetRendererBachelorThesis/Dataset_GameInstance.Materials` (`self.Materials`) _asdataset_game_instance)
  (set `/DatasetRendererBachelorThesis/Dataset_GameInstance.CameraPositions` (`self.CameraPositions`) _asdataset_game_instance)
  (set `/DatasetRendererBachelorThesis/Dataset_GameInstance.LightColors` (`self.LightColors`) _asdataset_game_instance)
  (bind _output_get_2 (set `/DatasetRendererBachelorThesis/Dataset_GameInstance.Index` 0 _asdataset_game_instance))
  (`GameplayStatics.OpenLevelBySoftObjectPtr` (`|GetArrayItem` _output_get _output_get_2)))

(fn `UserConstructionScript`)
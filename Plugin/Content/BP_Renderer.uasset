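; BP_Renderer drives dataset capture across a list of levels tracked by Dataset_GameInstance.
; After a fixed delay on BeginPlay, it increments the game instance's level index.
; It calls StartDatasetCapture at ObjectTargetPoint with the instance's cameras, light colors, materials, actor classes and fog setting.
; It passes the level at the new index as NextLevel, or null once the list is exhausted.
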(event `self.ReceiveBeginPlay`
  (`KismetSystemLibrary.Delay` 9.0)
  (bind _asdataset_game_instance (cast `/DatasetRendererBachelorThesis/Dataset_GameInstance` (`GameplayStatics.GetGameInstance`)))
  (bind _output_get (set `/DatasetRendererBachelorThesis/Dataset_GameInstance.Index` (+ (`/DatasetRendererBachelorThesis/Dataset_GameInstance.Index` _asdataset_game_instance) 1) _asdataset_game_instance))
  (bind _levels (`/DatasetRendererBachelorThesis/Dataset_GameInstance.Levels` _asdataset_game_instance))
  (if (< _output_get (`KismetArrayLibrary.Array_Length` _levels))
    (`BachelorRenderingBPLibrary.StartDatasetCapture` (`self.ObjectTargetPoint`) (`/DatasetRendererBachelorThesis/Dataset_GameInstance.CameraPositions` _asdataset_game_instance) (`/DatasetRendererBachelorThesis/Dataset_GameInstance.LightColors` _asdataset_game_instance) (`/DatasetRendererBachelorThesis/Dataset_GameInstance.Materials` _asdataset_game_instance) (`/DatasetRendererBachelorThesis/Dataset_GameInstance.ActorClass` _asdataset_game_instance) (`/DatasetRendererBachelorThesis/Dataset_GameInstance.AddFog` _asdataset_game_instance) (`|GetArrayItem` _levels (`/DatasetRendererBachelorThesis/Dataset_GameInstance.Index` _asdataset_game_instance)))
    (else
      (`BachelorRenderingBPLibrary.StartDatasetCapture` (`self.ObjectTargetPoint`) (`/DatasetRendererBachelorThesis/Dataset_GameInstance.CameraPositions` _asdataset_game_instance) (`/DatasetRendererBachelorThesis/Dataset_GameInstance.LightColors` _asdataset_game_instance) (`/DatasetRendererBachelorThesis/Dataset_GameInstance.Materials` _asdataset_game_instance) (`/DatasetRendererBachelorThesis/Dataset_GameInstance.ActorClass` _asdataset_game_instance) (`/DatasetRendererBachelorThesis/Dataset_GameInstance.AddFog` _asdataset_game_instance) (`self.NULL`)))))

(fn `UserConstructionScript`)